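; BP_Monster is the monster character in a Visitor pattern sample, showing a name and spoken messages in a widget above itself.
; On BeginPlay it adds a widget component raised above its origin, caches its WBP_SceneCharacterWidget and sets the header to the Russian word for "Monster".
; The Say event writes the incoming message into that widget's body text.
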(event `self.ReceiveBeginPlay`
  (bind _returnvalue (`AddComponent|NODE_AddWidgetComponent-0` :`RelativeTransform` (`KismetMathLibrary.MakeTransform` (0.0 0.0 100.0))))
  (bind _aswbp_scene_character_widget (cast `/Game/Patterns/Visitor/BP/WBP_SceneCharacterWidget` (`WidgetComponent.GetWidget` _returnvalue)))
  (bind _output_get (set `self.As WBP Scene Character Widget` _aswbp_scene_character_widget))
  (`TextBlock.SetText` (`/Game/Patterns/Visitor/BP/WBP_SceneCharacterWidget.Header` _output_get) "Монстр"))

(event `self.Say`
  (params (message :type String))
  (`TextBlock.SetText` (`/Game/Patterns/Visitor/BP/WBP_SceneCharacterWidget.Body` (`self.As WBP Scene Character Widget`)) (`KismetTextLibrary.Conv_StringToText` message)))

(fn `UserConstructionScript`)