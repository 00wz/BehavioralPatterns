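; Game mode for a Visitor pattern demo that applies a player-chosen visitor to every element in the level.
; On BeginPlay it caches all actors implementing IElement and shows a selection widget with MagicCristall, Potion and Trap buttons.
; Each click constructs the matching visitor object and passes it to VisitAll, which calls AcceptMessage on every cached actor.
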(event `self.ReceiveBeginPlay`
  (bind _outactors (`GameplayStatics.GetAllActorsWithInterface` "/Script/BehavioralPatterns.IElement"))
  (set `self.Out Actors` _outactors)
  (bind _returnvalue (`|CreateWidget` "/Game/Patterns/Visitor/BP/WBP_VisitorsSelectWidget.WBP_VisitorsSelectWidget_C"))
  (`UserWidget.AddToViewport` _returnvalue 0)
  (`|ExecutionSequence`
    (:`then_0`
      (add `Button.OnClicked` (`/Game/Patterns/Visitor/BP/WBP_VisitorsSelectWidget.MagicCristall` _returnvalue) (delegate `OnClicked_Event_0`)))
    (:`then_1`
      (add `Button.OnClicked` (`/Game/Patterns/Visitor/BP/WBP_VisitorsSelectWidget.Potion` _returnvalue) (delegate `OnClicked_Event_1`)))
    (:`then_2`
      (add `Button.OnClicked` (`/Game/Patterns/Visitor/BP/WBP_VisitorsSelectWidget.Trap` _returnvalue) (delegate `OnClicked_Event_2`)))))

(event `OnClicked_Event_0`
  (bind _returnvalue (`|GenericCreateObject` "/Script/BehavioralPatterns.MagicCrystal" self))
  (`self.VisitAll` _returnvalue))

(event `OnClicked_Event_1`
  (bind _returnvalue (`|GenericCreateObject` "/Script/BehavioralPatterns.Potion" self))
  (`self.VisitAll` _returnvalue))

(event `OnClicked_Event_2`
  (bind _returnvalue (`|GenericCreateObject` "/Script/BehavioralPatterns.Trap" self))
  (`self.VisitAll` _returnvalue))

(event `VisitAll`
  (params (NewParam :type "IVisitor Interface"))
  (for _array_element (`self.Out Actors`)
    (message `IElement.Accept` _array_element NewParam)))

(fn `UserConstructionScript`)