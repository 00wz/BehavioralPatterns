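; BP_Subject is the subject actor in an Observer pattern example, a clickable character that reports being attacked.
; On BeginPlay it adds a widget component above itself and sets the WBP_SceneCharacterWidget header to its Name.
; Clicking its mesh calls Notify with the Name joined to a Russian "attacked" message; Notify itself is defined outside this graph.
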(event `self.ReceiveBeginPlay`
  (bind _returnvalue (`AddComponent|NODE_AddWidgetComponent-1` :`RelativeTransform` (`KismetMathLibrary.MakeTransform` (0.0 0.0 100.0))))
  (bind _aswbp_scene_character_widget (cast `/Game/Patterns/Visitor/BP/WBP_SceneCharacterWidget` (`WidgetComponent.GetWidget` _returnvalue)))
  (`TextBlock.SetText` (`/Game/Patterns/Visitor/BP/WBP_SceneCharacterWidget.Header` _aswbp_scene_character_widget) (`self.Name`)))

(event `self.Mesh.OnClicked`
  (params (TouchedComponent :type "PrimitiveComponent Object Reference") (ButtonPressed :type "Key Structure"))
  (`Subject.Notify` (`KismetStringLibrary.Concat_StrStr` (`KismetTextLibrary.Conv_TextToString` (`self.Name`)) " атакован")))

(fn `UserConstructionScript`)