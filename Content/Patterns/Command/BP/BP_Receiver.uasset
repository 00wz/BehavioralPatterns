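; BP_Receiver is the receiver in a Command pattern example, a movable pawn that carries out timed directional moves.
; MoveRight, MoveLeft, MoveForward and MoveBack each pass a fixed world direction and the shared MoveDuration to MoveDirection.
; MoveDirection starts a timer bound to an empty event purely as a clock, then applies movement input each tick through a zero-delay loop while that timer is active.
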(event `MoveDirection`
  (params (Duration :type "Float (double-precision)") (Direction :type "Vector Structure"))
  (bind _returnvalue (`KismetSystemLibrary.K2_SetTimerDelegate` (delegate `Empty`) Duration))
  (if (`KismetSystemLibrary.K2_IsTimerActiveHandle` _returnvalue) :!label _label
    (`KismetSystemLibrary.Delay` 0.0)
    (`self.AddMovementInput` Direction)
    (goto _label)))

(event `Empty`)

(event `self.MoveRight`
  (`self.MoveDirection` (`self.MoveDuration`) (`KismetMathLibrary.Vector_Right`)))

(event `self.MoveLeft`
  (`self.MoveDirection` (`self.MoveDuration`) (`KismetMathLibrary.Vector_Left`)))

(event `self.MoveForward`
  (`self.MoveDirection` (`self.MoveDuration`) (`KismetMathLibrary.Vector_Forward`)))

(event `self.MoveBack`
  (`self.MoveDirection` (`self.MoveDuration`) (`KismetMathLibrary.Vector_Backward`)))

(fn `UserConstructionScript`)